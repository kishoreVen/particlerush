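; BP_Rush is the Blueprint for Rush, a winged craft or character with boost effects.
; Its construction script attaches effect components to left thrust, right thrust and core sockets on the main mesh, then snaps a shared wing skeletal mesh onto both wing sockets.
; Boost stage-up events activate two components, resetting only the first, and boost end deactivates two.
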(event `self.OnBoostStageUp`
  (params (stage :type Integer))
  ;[1 1 1] Boost Events
  (`ActorComponent.Activate` true)
  (`ActorComponent.Activate` false))

(event `self.OnBoostEnd`
  ;[1 1 1] Boost Events
  (`ActorComponent.Deactivate`)
  (`ActorComponent.Deactivate`))

(fn `InitializeParticleSystems`
  (bind _mesh (`self.Mesh`))
  (`SceneComponent.K2_AttachTo` _mesh "thrust_left_socket" "SnapToTarget" false)
  (`SceneComponent.K2_AttachTo` _mesh "thrust_right_socket" "SnapToTarget" false)
  (`SceneComponent.K2_AttachTo` _mesh "Core_Socket"))

(fn `UserConstructionScript`
  (bind _leftwingmesh (`self.LeftWingMesh`))
  (bind _rightwingmesh (`self.RightWingMesh`))
  (bind _mesh (`self.Mesh`))
  (`self.InitializeParticleSystems`)
  (`SkinnedMeshComponent.SetSkinnedAssetAndUpdate` _leftwingmesh "/Game/Assets/Rush/Import/Wings/skeletalmesh_Rush_wing.skeletalmesh_Rush_wing")
  (`SceneComponent.K2_AttachTo` _leftwingmesh _mesh "LeftWingSocket" "SnapToTarget" true)
  (`SkinnedMeshComponent.SetSkinnedAssetAndUpdate` _rightwingmesh "/Game/Assets/Rush/Import/Wings/skeletalmesh_Rush_wing.skeletalmesh_Rush_wing")
  (`SceneComponent.K2_AttachTo` _rightwingmesh _mesh "RightWingSocket" "SnapToTarget" true))