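; Base spline track actor that builds an accelerator track from spline meshes in its construction script.
; It first syncs a per-point track data array to the spline's point count, matching stored point locations to find entries to remove.
; It then adds a main mesh per segment, plus a tunnel mesh where flagged, blending banking and scale between points.
; A looping flag adds the segment closing back to the first point.
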(event EventBeginPlay)

(event Collision|EventActorBeginOverlap
  (params (OtherActor :type Actor%20Object%20Reference)))

(event EventTick
  (params (DeltaSeconds :type Float%20%28single-precision%29)))

(fn ConstructionScript
  (|SyncTrackDataandSpline
    (:Exec
      (|BuildtheTrack))))

(fn AddTrackElement
  (params (Mesh :type Static%20Mesh%20Object%20Reference) (Index :type Integer))
  (bind (_start_location _start_tangent _end_location _end_tangent _start_track_data _end_track_data) (|FetchSplineData Index)
    (:Exec
      (bind _returnvalue (AddComponent|AddSplineMeshComponent false))
      (Components|StaticMesh|SetStaticMesh _returnvalue Mesh)
      (SplineMesh|SetStartandEnd _returnvalue _start_location _start_tangent _end_location _end_tangent :!class /Script/Engine.SplineMeshComponent)
      (Class|SplineMeshComponent|SetStartRoll _returnvalue (.BankingAngle (Utilities|Struct|BreakTrackData _start_track_data)))
      (Class|SplineMeshComponent|SetEndRoll _returnvalue (.BankingAngle (Utilities|Struct|BreakTrackData _end_track_data)))
      (SplineMesh|SetStartScale _returnvalue (.TrackScale (Utilities|Struct|BreakTrackData _start_track_data)) :!class /Script/Engine.SplineMeshComponent)
      (SplineMesh|SetEndScale _returnvalue (.TrackScale (Utilities|Struct|BreakTrackData _end_track_data)) :!class /Script/Engine.SplineMeshComponent))))