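; BP_WallGenerator is a construction-script actor that builds a straight wall or fence of repeated meshes from its origin toward EndPoint.
; It divides the horizontal distance to EndPoint by MeshWidth and rounds it to get the segment count.
; Extra MeshToSpawn components attach to FenceStart, spaced along its local X axis.
; FenceStart then yaws toward EndPoint, turning the whole row while ignoring height differences.
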(event `self.ReceiveBeginPlay`)

(event `self.ReceiveActorBeginOverlap`
  (params (OtherActor :type "Actor Object Reference")))

(event `self.ReceiveTick`
  (params (DeltaSeconds :type "Float (single-precision)")))

(fn `UserConstructionScript`
  (bind _returnvalue (`self.K2_GetActorLocation`))
  (bind _returnvalue_2 (- (`KismetMathLibrary.Round` (/ (`KismetMathLibrary.VSize` (* (`self.EndPoint`) (1.0 1.0 0.0))) (`self.MeshWidth`))) 1))
  (`StaticMeshComponent.SetStaticMesh` (`self.FenceStart`) (`self.MeshToSpawn`)) ; Change spawned mesh to the new type
  (if (> _returnvalue_2 0)
    (for _index (range 1 (+ _returnvalue_2 1))
      (bind _returnvalue_3 (`AddComponent|StaticMeshComponent_5` :`bManualAttachment` true))
      (`SceneComponent.K2_AttachTo` _returnvalue_3 (`self.FenceStart`) "None" "KeepWorldPosition" true) ; Attach each segment to the initial mesh
      (`SceneComponent.K2_SetRelativeLocation` _returnvalue_3 (`KismetMathLibrary.MakeVector` (* _index (`self.MeshWidth`))) false)
      (`StaticMeshComponent.SetStaticMesh` _returnvalue_3 (`self.MeshToSpawn`)) ; Change spawned mesh to the new type
    ))
  (`SceneComponent.K2_SetWorldRotation` (`self.FenceStart`) (`KismetMathLibrary.MakeRot` 0.0 (.yaw (`KismetMathLibrary.FindLookAtRotation` _returnvalue (+ _returnvalue (`self.EndPoint`))))) false) ; Rotate the initial mesh to face the end point
)