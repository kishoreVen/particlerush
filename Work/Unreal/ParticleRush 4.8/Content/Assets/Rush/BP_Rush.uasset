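; BP_Rush is the Rush craft actor, assembling a winged skeletal mesh with thruster and core effects and driving their boost feedback.
; Construction snaps the wings, thrust audio and particle systems to mesh sockets.
; Boost stage-up events trigger the thruster effects and feed the normalized stage into both thrust sounds; boost end deactivates effects.
; The core cue starts on BeginPlay, then switches its AudioType parameter and replays when the first phase finishes.
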(event `self.ReceiveBeginPlay`
  (bind _coreaudiocomponent (`self.CoreAudioComponent`))
  (set `AudioComponent.Sound` "/Game/Assets/Rush/Audio/Cue/ucue_rush_core.ucue_rush_core" _coreaudiocomponent)
  (`AudioComponent.SetIntParameter` "AudioType")
  (`AudioComponent.Play` _coreaudiocomponent 0.0))

(event `self.ReceiveTick`
  (params (DeltaSeconds :type "Float (single-precision)")))

(event `self.OnBoostStageUp`
  (params (stage :type Integer) (normalizedStage :type "Float (single-precision)"))
  ;[1 1 1] Boost Events
  (`ActorComponent.Activate` true)
  (`ActorComponent.Activate` false)
  (`AudioComponent.SetFloatParameter` (`self.RightThrustAudio`) "BoostStage" normalizedStage)
  (`AudioComponent.SetFloatParameter` (`self.LeftThrustAudio`) "BoostStage" normalizedStage)
  (`AudioComponent.Play` 0.0)
  (`AudioComponent.Play` 0.0))

(event `self.OnBoostEnd`
  ;[1 1 1] Boost Events
  (`ActorComponent.Deactivate`)
  (`ActorComponent.Deactivate`))

(event `self.CoreAudioComponent.OnAudioFinished`
  (if (`|EnumEquality` (`self.CoreAudioType`) "NewEnumerator0")
    (set `self.CoreAudioType` "NewEnumerator1")
    (`AudioComponent.SetIntParameter` "AudioType" 1)
    (`AudioComponent.Play` 0.0)))

(fn `InitializeAudioSystems`
  (bind _mesh (`self.Mesh`))
  (`SceneComponent.K2_AttachTo` _mesh "thrust_left_socket" "SnapToTarget" false)
  (`SceneComponent.K2_AttachTo` _mesh "thrust_right_socket" "SnapToTarget" false))

(fn `InitializeParticleSystems`
  (bind _mesh (`self.Mesh`))
  (`SceneComponent.K2_AttachTo` _mesh "thrust_left_socket" "SnapToTarget" false)
  (`SceneComponent.K2_AttachTo` _mesh "thrust_right_socket" "SnapToTarget" false)
  (`SceneComponent.K2_AttachTo` _mesh "Core_Socket"))

(fn `UserConstructionScript`
  (bind _leftwingmesh (`self.LeftWingMesh`))
  (bind _rightwingmesh (`self.RightWingMesh`))
  (bind _mesh (`self.Mesh`))
  (`self.InitializeParticleSystems`)
  (`self.InitializeAudioSystems`)
  (`SkinnedMeshComponent.SetSkinnedAssetAndUpdate` _leftwingmesh "/Game/Assets/Rush/Import/Wings/skeletalmesh_Rush_wing.skeletalmesh_Rush_wing")
  (`SceneComponent.K2_AttachTo` _leftwingmesh _mesh "LeftWingSocket" "SnapToTarget" true)
  (`SkinnedMeshComponent.SetSkinnedAssetAndUpdate` _rightwingmesh "/Game/Assets/Rush/Import/Wings/skeletalmesh_Rush_wing.skeletalmesh_Rush_wing")
  (`SceneComponent.K2_AttachTo` _rightwingmesh _mesh "RightWingSocket" "SnapToTarget" true))